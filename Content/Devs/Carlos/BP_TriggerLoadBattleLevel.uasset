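; Trigger actor that starts a battle level when the player character overlaps its box.
; On overlap by BP_ThirdPersonCharacter, it passes its configured level asset, three enemy classes and floor mesh to the BattleLevelManager, which loads and configures the level.
; A debug "Hello" print fires on trigger, and a direct stream-level load node is left disconnected.
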(event `self.Box.OnComponentBeginOverlap`
  (params (OverlappedComponent :type "PrimitiveComponent Object Reference") (OtherActor :type "Actor Object Reference") (OtherComp :type "PrimitiveComponent Object Reference") (OtherBodyIndex :type Integer) (bFromSweep :type Boolean) (SweepResult :type "HitResult Structure (by ref)"))
  (cast `/Game/ThirdPerson/Blueprints/BP_ThirdPersonCharacter` OtherActor)
  (`KismetSystemLibrary.PrintText` "Hello")
  (`BattleLevelManager.LoadAndConfigureBattleLevel` (subsystem `BattleLevelManager`) (`self.BattleLevelToLoad`) (`self.EnemyAClass`) (`self.EnemyBClass`) (`self.EnemyCClass`) (`self.MeshFloor`)))

(fn `UserConstructionScript`)